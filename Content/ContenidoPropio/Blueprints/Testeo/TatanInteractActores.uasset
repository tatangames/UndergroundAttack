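; Interaction point for "Tatan", used as a child actor, that notifies its parent actor through ActivarTatanObjeto when triggered, optionally only once until re-enabled.
; Enable and disable events toggle its Sphere collision and active state.
; The Box detects the player and fades a TatanInteractIcon widget through target opacities.
; On exit, a retriggerable delay polls until the icon is transparent, then removes it.
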(event `/Game/ContenidoPropio/Blueprints/Testeo/TatanInterfaceBP.EnableTatanInteract`
  (`self.ResetDoOnce`)
  (set `self.Activated` true)
  (`PrimitiveComponent.SetCollisionEnabled` (`self.Sphere`) "QueryAndPhysics")
  (`self.PopulateIconWidget`)
  (set `/Game/ContenidoPropio/Blueprints/Testeo/TatanInteractIcon.TatanTargetActivatedOpacity` 1.0 (`self.TatanIconRef`))
  (`/Engine/EditorBlueprintResources/StandardMacros.IsValid` (`|GetArrayItem` (`PrimitiveComponent.GetOverlappingActors` (`self.Box`) "/Game/FirstPerson/Blueprints/BP_FirstPersonCharacter.BP_FirstPersonCharacter_C"))
    (:`Is Valid`
      (set `/Game/ContenidoPropio/Blueprints/Testeo/TatanInteractIcon.TatanNearBoxTriggerTargetOpacity` 1.0 (`self.TatanIconRef`)))))

(event `PopulateIconWidget`
  (bind _tataniconref (`self.TatanIconRef`))
  (`/Engine/EditorBlueprintResources/StandardMacros.IsValid` (`self.TatanIconRef`)
    (:`Is Not Valid`
      (bind _returnvalue (`|CreateWidget` "/Game/ContenidoPropio/Blueprints/Testeo/TatanInteractIcon.TatanInteractIcon_C"))
      (set `self.TatanIconRef` _returnvalue)
      (set `/Game/ContenidoPropio/Blueprints/Testeo/TatanInteractIcon.ParentActor` self (`self.TatanIconRef`))
      (`UserWidget.AddToViewport` _tataniconref -1)
      (`UserWidget.SetDesiredSizeInViewport` _tataniconref (32.0 32.0))
      (set `/Game/ContenidoPropio/Blueprints/Testeo/TatanInteractIcon.TatanNearBoxTriggerTargetOpacity` 0.0 (`self.TatanIconRef`)))))

(event `/Game/ContenidoPropio/Blueprints/Testeo/TatanInterfaceBP.DisableCoroInteract`
  (set `self.Activated` false)
  (`PrimitiveComponent.SetCollisionEnabled` (`self.Sphere`) "NoCollision")
  (set `/Game/ContenidoPropio/Blueprints/Testeo/TatanInteractIcon.TatanTargetActivatedOpacity` 0.0 (`self.TatanIconRef`)))

(event `self.ReceiveBeginPlay`
  (if (`self.Activated`)
    (`KismetSystemLibrary.Delay` 0.2)
    (`/Engine/EditorBlueprintResources/StandardMacros.IsValid` (`|GetArrayItem` (`PrimitiveComponent.GetOverlappingActors` (`self.Box`) "/Game/FirstPerson/Blueprints/BP_FirstPersonCharacter.BP_FirstPersonCharacter_C"))
      (:`Is Valid`
        (`self.PopulateIconWidget`)
        (set `/Game/ContenidoPropio/Blueprints/Testeo/TatanInteractIcon.TatanNearBoxTriggerTargetOpacity` 1.0 (`self.TatanIconRef`))))
    (else
      (`PrimitiveComponent.SetCollisionEnabled` (`self.Sphere`) "NoCollision"))))

(event `ResetDoOnce`
  (goto _label :!via `Reset`))

(event `/Game/ContenidoPropio/Blueprints/Testeo/TatanInterfaceBP.ActivarTatanChildActor`
  (bind _returnvalue (`self.GetParentActor`))
  (`/Engine/EditorBlueprintResources/StandardMacros.IsValid` _returnvalue
    (:`Is Valid`
      (if (`self.Activated`)
        (if (`self.DoOnce`)
          (`/Engine/EditorBlueprintResources/StandardMacros.DoOnce` false :!label _label
            (:`Completed`
              (message `/Game/ContenidoPropio/Blueprints/Testeo/TatanInterfaceBP.ActivarTatanObjeto` _returnvalue)
              (`PrimitiveComponent.SetCollisionEnabled` (`self.Sphere`) "NoCollision")
              (set `/Game/ContenidoPropio/Blueprints/Testeo/TatanInteractIcon.TatanTargetActivatedOpacity` 0.0 (`self.TatanIconRef`))
              (set `self.Activated` false)))
          (else
            (message `/Game/ContenidoPropio/Blueprints/Testeo/TatanInterfaceBP.ActivarTatanObjeto` _returnvalue)))))))

(event `self.Box.OnComponentBeginOverlap`
  (params (OverlappedComponent :type "PrimitiveComponent Object Reference") (OtherActor :type "Actor Object Reference") (OtherComp :type "PrimitiveComponent Object Reference") (OtherBodyIndex :type Integer) (bFromSweep :type Boolean) (SweepResult :type "HitResult Structure (by ref)"))
  (if (`self.ActorHasTag` OtherActor "Player")
    (set `self.IsPlayerNearTrigger` true)
    (if (`self.Activated`)
      (`self.PopulateIconWidget`)
      (set `/Game/ContenidoPropio/Blueprints/Testeo/TatanInteractIcon.TatanNearBoxTriggerTargetOpacity` 1.0 (`self.TatanIconRef`)))))

(event `self.Box.OnComponentEndOverlap`
  (params (OverlappedComponent :type "PrimitiveComponent Object Reference") (OtherActor :type "Actor Object Reference") (OtherComp :type "PrimitiveComponent Object Reference") (OtherBodyIndex :type Integer))
  (if (`self.ActorHasTag` OtherActor "Player")
    (set `self.IsPlayerNearTrigger` false)
    (`/Engine/EditorBlueprintResources/StandardMacros.IsValid` (`self.TatanIconRef`)
      (:`Is Valid`
        (set `/Game/ContenidoPropio/Blueprints/Testeo/TatanInteractIcon.TatanNearBoxTriggerTargetOpacity` 0.0 (`self.TatanIconRef`))
        (`KismetSystemLibrary.RetriggerableDelay` 0.2 :!label _label_2)
        (if (`self.IsPlayerNearTrigger`)
          _
          (elif (`KismetMathLibrary.NearlyEqual_FloatFloat` (`/Game/ContenidoPropio/Blueprints/Testeo/TatanInteractIcon.TotalOpacity` (`self.TatanIconRef`)))
            (`Widget.RemoveFromParent` (`self.TatanIconRef`))
            (set `self.TatanIconRef` null)
            (else
              (goto _label_2))))))))

(fn `UserConstructionScript`)