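; Interactable door that swings open and closed, and can be locked behind a key object.
; ActivarTatanObjeto checks KeyToUnlock: while it is valid, the player sees a "needs a key" message and the door plays a slight rattle.
; Otherwise, a FlipFlop plays or reverses a timeline that yaws the door's Scene component.
; The construction script copies TatanChildConfig into the child TatanInteractActores, setting its prompt, trigger sizes and activation flags.
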(event `/Game/ContenidoPropio/Blueprints/Testeo/TatanInterfaceBP.ActivarTatanObjeto`
  (`/Engine/EditorBlueprintResources/StandardMacros.IsValid` (`self.KeyToUnlock`)
    (:`Is Valid`
      (`/Game/FirstPerson/Blueprints/BP_FirstPersonCharacter.MostrarAnuncio` (cast `/Game/FirstPerson/Blueprints/BP_FirstPersonCharacter` (`GameplayStatics.GetPlayerCharacter` 0) :!pure true) "Necesitas una llave" 5.0)
      (bind (_direction _animpuertaconllave) (`Timeline|Timeline_0` :!via `PlayFromStart`)
        (:`Update`
          (`SceneComponent.K2_SetRelativeRotation` (`self.Scene`) (`KismetMathLibrary.MakeRotator` 0.0 0.0 (`KismetMathLibrary.Lerp` 0.0 2.5 _animpuertaconllave)) false false))))
    (:`Is Not Valid`
      (`/Engine/EditorBlueprintResources/StandardMacros.FlipFlop`
        (:`A`
          (bind (_direction_2 _newtrack_0) (`Timeline|Timeline` :!label _label)
            (:`Update`
              (`SceneComponent.K2_SetRelativeRotation` (`self.Scene`) (`KismetMathLibrary.MakeRotator` 0.0 0.0 (`KismetMathLibrary.Lerp` 0.0 110.0 _newtrack_0)) false false))))
        (:`B`
          (goto _label :!via `Reverse`))))))

(fn `UserConstructionScript`
  (bind (_tatanname _tatansphereradio _hacerunavez _empiezaactivo _triggersize) (break `/Game/ContenidoPropio/Blueprints/Testeo/TatanChildStructure` (`self.Tatan Child Config`)))
  (bind _astatan_interact_actores (cast `/Game/ContenidoPropio/Blueprints/Testeo/TatanInteractActores` (`ChildActorComponent.ChildActor` (`self.ChildActor1`)) :!pure true))
  (set `/Game/ContenidoPropio/Blueprints/Testeo/TatanInteractActores.InteractText` _tatanname _astatan_interact_actores)
  (`SphereComponent.SetSphereRadius` (`/Game/ContenidoPropio/Blueprints/Testeo/TatanInteractActores.Sphere` _astatan_interact_actores) _tatansphereradio true)
  (set `/Game/ContenidoPropio/Blueprints/Testeo/TatanInteractActores.DoOnce` _hacerunavez _astatan_interact_actores)
  (set `/Game/ContenidoPropio/Blueprints/Testeo/TatanInteractActores.Activated` _empiezaactivo _astatan_interact_actores)
  (`BoxComponent.SetBoxExtent` (`/Game/ContenidoPropio/Blueprints/Testeo/TatanInteractActores.Box` _astatan_interact_actores) _triggersize true))