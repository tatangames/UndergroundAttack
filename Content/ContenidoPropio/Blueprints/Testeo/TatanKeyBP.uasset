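; TatanKeyBP is a key pickup actor, in a testing folder, with interaction delegated to a TatanInteractActores child actor.
; The construction script pushes TatanChildConfig into that child: prompt text, sphere and box sizes, do-once and initial active state.
; ActivarTatanObjeto disables the child's interaction, then hides the key and its collision instead of destroying it.
; BeginPlay stores the spawn location and debug-prints it.
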(event `self.ReceiveBeginPlay`
  (bind _returnvalue (`self.K2_GetActorLocation`))
  (set `self.SpawnLocalizacion` _returnvalue)
  (`KismetSystemLibrary.PrintString` (`KismetStringLibrary.Conv_VectorToString` _returnvalue) true true (struct :`G` 0.66 :`B` 1.0 :`A` 1.0) 60.0))

(event `/Game/ContenidoPropio/Blueprints/Testeo/TatanInterfaceBP.ActivarTatanObjeto`
  (`/Game/ContenidoPropio/Blueprints/Testeo/TatanInterfaceBP.DisableTatanInteract` (cast `/Game/ContenidoPropio/Blueprints/Testeo/TatanInteractActores` (`ChildActorComponent.ChildActor` (`self.ChildActor1`)) :!pure true))
  (`self.SetActorHiddenInGame` true)
  (`self.SetActorEnableCollision` false))

(fn `UserConstructionScript`
  (bind (_tatanname _tatansphereradio _hacerunavez _empiezaactivo _triggersize) (break `/Game/ContenidoPropio/Blueprints/Testeo/TatanChildStructure` (`self.TatanChildConfig`)))
  (bind _astatan_interact_actores (cast `/Game/ContenidoPropio/Blueprints/Testeo/TatanInteractActores` (`ChildActorComponent.ChildActor` (`self.ChildActor1`)) :!pure true))
  (set `/Game/ContenidoPropio/Blueprints/Testeo/TatanInteractActores.InteractText` _tatanname _astatan_interact_actores)
  (`SphereComponent.SetSphereRadius` (`/Game/ContenidoPropio/Blueprints/Testeo/TatanInteractActores.Sphere` _astatan_interact_actores) _tatansphereradio true)
  (set `/Game/ContenidoPropio/Blueprints/Testeo/TatanInteractActores.DoOnce` _hacerunavez _astatan_interact_actores)
  (set `/Game/ContenidoPropio/Blueprints/Testeo/TatanInteractActores.Activated` _empiezaactivo _astatan_interact_actores)
  (`BoxComponent.SetBoxExtent` (`/Game/ContenidoPropio/Blueprints/Testeo/TatanInteractActores.Box` _astatan_interact_actores) _triggersize true))