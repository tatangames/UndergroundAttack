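; BP_Puerta is a test door that opens when the ActivarTatanObjeto event fires, snapping its Scene component to a fixed relative rotation with no animation or closing logic.
; The Construction Script copies TatanChildConfig into its TatanInteractActores child actor, setting interaction text, sphere radius, trigger box size, do-once and initial active state.
; The event's caller is outside this Blueprint.
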(event `/Game/ContenidoPropio/Blueprints/Testeo/TatanInterfaceBP.ActivarTatanObjeto`
  (`SceneComponent.K2_SetRelativeRotation` (`self.Scene`) (struct :`Yaw` 90.0) false false))

(fn `UserConstructionScript`
  (bind (_tatanname _tatansphereradio _hacerunavez _empiezaactivo _triggersize) (break `/Game/ContenidoPropio/Blueprints/Testeo/TatanChildStructure` (`self.TatanChildConfig`)))
  (bind _astatan_interact_actores (cast `/Game/ContenidoPropio/Blueprints/Testeo/TatanInteractActores` (`ChildActorComponent.ChildActor` (`self.ChildActor1`)) :!pure true))
  (set `/Game/ContenidoPropio/Blueprints/Testeo/TatanInteractActores.InteractText` _tatanname _astatan_interact_actores)
  (`SphereComponent.SetSphereRadius` (`/Game/ContenidoPropio/Blueprints/Testeo/TatanInteractActores.Sphere` _astatan_interact_actores) _tatansphereradio true)
  (set `/Game/ContenidoPropio/Blueprints/Testeo/TatanInteractActores.DoOnce` _hacerunavez _astatan_interact_actores)
  (set `/Game/ContenidoPropio/Blueprints/Testeo/TatanInteractActores.Activated` _empiezaactivo _astatan_interact_actores)
  (`BoxComponent.SetBoxExtent` (`/Game/ContenidoPropio/Blueprints/Testeo/TatanInteractActores.Box` _astatan_interact_actores) _triggersize true))