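; MiTrigger is a reusable box trigger that fires MiTriggerDispatcher when an actor carrying the player tag overlaps it.
; Overlaps count only while Activado is set, and the overlapping actor is stored before the dispatcher call.
; UnaVezBool routes the call through a DoOnce gate, which ActivarTrigger resets when re-enabling the trigger; DesactivarTrigger disables it.
; The construction script applies the configurable box size and description text.
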(event `DesactivarTrigger`
  (set `self.Activado` false))

(event `ActivarTrigger`
  (`self.ResetearDoOnce`)
  (set `self.Activado` true))

(event `ResetearDoOnce`
  (goto _label :!via `Reset`))

(event `self.Box.OnComponentBeginOverlap`
  (params (OverlappedComponent :type "PrimitiveComponent Object Reference") (OtherActor :type "Actor Object Reference") (OtherComp :type "PrimitiveComponent Object Reference") (OtherBodyIndex :type Integer) (bFromSweep :type Boolean) (SweepResult :type "HitResult Structure (by ref)"))
  (if (`self.Activado`)
    (if (`self.ActorHasTag` OtherActor (`self.EtiquetaPlayer`))
      (set `self.ActorWhoActivatedTheTrigger` OtherActor)
      (if (`self.UnaVezBool`)
        (`/Engine/EditorBlueprintResources/StandardMacros.DoOnce` false :!label _label
          (:`Completed`
            _)))
      (`self.MiTriggerDispatcher`))))

(fn `UserConstructionScript`
  (`BoxComponent.SetBoxExtent` (`self.Box`) (`self.TamanoDelTrigger`) true)
  (`TextRenderComponent.K2_SetText` (`self.TextRender`) (`self.DescripcionTrigger`)))