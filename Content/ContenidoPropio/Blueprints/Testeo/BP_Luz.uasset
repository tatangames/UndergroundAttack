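; BP_Luz is an interactable light whose point light toggles on and off through the Tatan interaction system.
; ActivarTatanObjeto calls the ButtonActivated dispatcher, then uses a FlipFlop to hide and show the PointLight, hiding it on the first activation.
; The construction script passes TatanChildConfig to TatanConstruct, which configures the TatanInteractActores child actor's prompt text, trigger sizes, do-once flag and initial active state.
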(event `/Game/ContenidoPropio/Blueprints/Testeo/TatanInterfaceBP.ActivarTatanObjeto`
  (`self.ButtonActivatedDispachador`)
  (`/Engine/EditorBlueprintResources/StandardMacros.FlipFlop`
    (:`A`
      (`SceneComponent.SetHiddenInGame` (`self.PointLight`) true false))
    (:`B`
      (`SceneComponent.SetHiddenInGame` (`self.PointLight`) false false))))

(event `vfsgvdfv`)

(fn `UserConstructionScript`
  (bind (_tatanname _tatansphereradio _hacerunavez _empiezaactivo _triggersize) (break `/Game/ContenidoPropio/Blueprints/Testeo/TatanChildStructure` (`self.TatanChildConfig`)))
  (bind _astatan_interact_actores (cast `/Game/ContenidoPropio/Blueprints/Testeo/TatanInteractActores` (`ChildActorComponent.ChildActor` (`self.ChildActor1`)) :!pure true))
  (set `/Game/ContenidoPropio/Blueprints/Testeo/TatanInteractActores.InteractText` _tatanname _astatan_interact_actores)
  (`SphereComponent.SetSphereRadius` (`/Game/ContenidoPropio/Blueprints/Testeo/TatanInteractActores.Sphere` _astatan_interact_actores) _tatansphereradio true)
  (set `/Game/ContenidoPropio/Blueprints/Testeo/TatanInteractActores.DoOnce` _hacerunavez _astatan_interact_actores)
  (set `/Game/ContenidoPropio/Blueprints/Testeo/TatanInteractActores.Activated` _empiezaactivo _astatan_interact_actores)
  (`BoxComponent.SetBoxExtent` (`/Game/ContenidoPropio/Blueprints/Testeo/TatanInteractActores.Box` _astatan_interact_actores) _triggersize true))