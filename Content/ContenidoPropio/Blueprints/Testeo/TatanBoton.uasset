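; TatanBoton is an interactable button actor that sinks when activated.
; The construction script pushes the TatanChildConfig struct into its TatanInteractActores child actor, setting prompt text, sphere and box trigger sizes, do-once and initial active state.
; ActivarTatanObjeto plays a timeline from the start that lerps the Scene component 50 units down from its relative origin.
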(event `/Game/ContenidoPropio/Blueprints/Testeo/TatanInterfaceBP.ActivarTatanObjeto`
  (bind (_direction _newtrack_0) (`Timeline|Timeline` :!via `PlayFromStart`)
    (:`Update`
      (`SceneComponent.K2_SetRelativeLocation` (`self.Scene`) (`KismetMathLibrary.VLerp` (0.0 0.0 0.0) (0.0 0.0 -50.0) _newtrack_0) false false))))

(fn `UserConstructionScript`
  (bind (_tatanname _tatansphereradio _hacerunavez _empiezaactivo _triggersize) (break `/Game/ContenidoPropio/Blueprints/Testeo/TatanChildStructure` (`self.Tatan Child Config`)))
  (bind _astatan_interact_actores (cast `/Game/ContenidoPropio/Blueprints/Testeo/TatanInteractActores` (`ChildActorComponent.ChildActor` (`self.ChildActor`)) :!pure true))
  (set `/Game/ContenidoPropio/Blueprints/Testeo/TatanInteractActores.InteractText` _tatanname _astatan_interact_actores)
  (`SphereComponent.SetSphereRadius` (`/Game/ContenidoPropio/Blueprints/Testeo/TatanInteractActores.Sphere` _astatan_interact_actores) _tatansphereradio true)
  (set `/Game/ContenidoPropio/Blueprints/Testeo/TatanInteractActores.DoOnce` _hacerunavez _astatan_interact_actores)
  (set `/Game/ContenidoPropio/Blueprints/Testeo/TatanInteractActores.Activated` _empiezaactivo _astatan_interact_actores)
  (`BoxComponent.SetBoxExtent` (`/Game/ContenidoPropio/Blueprints/Testeo/TatanInteractActores.Box` _astatan_interact_actores) _triggersize true))